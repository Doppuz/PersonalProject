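; Skeleton melee emerge action that runs cleanup when the enemy's emerge ends.
; On stop, the authority stops the Invincible action on the owner and sets the HasEmerged key on the AI controller's blackboard to true.
; The action then removes itself from the owner's action component.
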(event `self.StopAction`
  (params (Instigator :type "Actor Object Reference"))
  (bind _actioncomponentowner (`self.ActionComponentOwner`))
  (bind _returnvalue (`ActorComponent.GetOwner` _actioncomponentowner))
  (`parent.StopAction` null)
  (if (`Actor.HasAuthority` _returnvalue)
    (bind _aspawn (cast `Pawn` _returnvalue))
    (bind _asbase_aicontroller (cast `BaseAIController` (`AIBlueprintHelperLibrary.GetAIController` _aspawn)))
    (`ActionComponent.StopActionByName` _actioncomponentowner null (struct :`TagName` "Action.Invincible"))
    (`BlackboardComponent.SetValueAsBool` (`AIBlueprintHelperLibrary.GetBlackboard` _asbase_aicontroller) (`self.HasEmergedKey`) true)
    (`ActionComponent.RemoveAction` (`self.ActionComponentOwner`) null self)))